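; HUD Blueprint for the shooting game that relays the local player's HP, ammo and magazine values to ShootingHudWidget.
; User name and kill/death updates rebuild the widget's player list sorted by kills, with kill/death changes also printed on screen as debug text.
; UpdateHud refreshes that list, re-arming itself on a short timer until the HUD widget cast succeeds.
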(event EventOnUpdateKillDeath
  (params (kill :type Integer) (death :type Integer))
  (Development|PrintString (Utilities|String|Append "Update Kill : " (Utilities|String|ToString(Integer) kill) ", Death : " (Utilities|String|ToString(Integer) death)) true true "(R=0.000000,G=0.660000,B=1.000000,A=1.000000)" 6e+01)
  (bind _asshooting_hud_widget (Utilities|Casting|CastToShootingHudWidget (Variables|Default|GetHudWidget)))
  (Default|UpdatePlayerList _asshooting_hud_widget (Class|ShootingHUD|GetPlayerListSortbyKill)))

(event EventOnUpdateMyAmmo
  (params (Ammo :type Integer))
  (bind _asshooting_hud_widget (Utilities|Casting|CastToShootingHudWidget (Variables|Default|GetHudWidget)))
  (Default|SetAmmo _asshooting_hud_widget Ammo))

(event EventOnUpdateMyMag
  (params (Mag :type Integer))
  (bind _asshooting_hud_widget (Utilities|Casting|CastToShootingHudWidget (Variables|Default|GetHudWidget)))
  (Default|SetMag _asshooting_hud_widget Mag))

(event EventOnUpdateMyHp
  (params (CurHp :type Float%20%28single-precision%29) (MaxHp :type Float%20%28single-precision%29))
  (bind _asshooting_hud_widget (Utilities|Casting|CastToShootingHudWidget (Variables|Default|GetHudWidget)))
  (Default|SetHp _asshooting_hud_widget CurHp MaxHp))

(event EventOnUpdateUserName
  (params (userName :type String))
  (bind _asshooting_hud_widget (Utilities|Casting|CastToShootingHudWidget (Variables|Default|GetHudWidget)))
  (Default|UpdatePlayerList _asshooting_hud_widget (Class|ShootingHUD|GetPlayerListSortbyKill)))

(fn ConstructionScript)

(fn UpdateHud
  (bind _asshooting_hud_widget (Utilities|Casting|CastToShootingHudWidget (Variables|Default|GetHudWidget))
    (:then
      (Default|UpdatePlayerList _asshooting_hud_widget (Class|ShootingHUD|GetPlayerListSortbyKill)))
    (:CastFailed
      (Utilities|Time|SetTimerbyFunctionName 0 "UpdateHud" 0.1))))