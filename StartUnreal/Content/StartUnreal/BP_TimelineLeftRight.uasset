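; Actor Blueprint that slides its Sphere component back and forth along its relative X axis with a timeline, as a child of a class providing play/stop control.
; DoPlay calls the parent version, then EventStart, which plays or reverses the timeline according to IsMoveRight.
; Timeline updates scale the value into the sphere's X position, and finishing flips IsMoveRight and loops back for continuous ping-pong motion.
; DoStop halts the timeline.
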(event Custom|DoStop
  (bind _value (Timeline|타임라인 Stop)
    (:Update
      (Transformation|SetRelativeLocation (Variables|Default|GetSphere) (Math|Vector|MakeVector (* _value 1e+02) 0.0 0.0) false false))
    (:Finished
      (Variables|Default|SetIsMoveRight (not (Variables|Default|GetIsMoveRight)))
      (if (Variables|Default|GetIsMoveRight)
        (Timeline|타임라인 Play)
        (else
          (Timeline|타임라인 Reverse))))))

(event Custom|EventStart
  (if (Variables|Default|GetIsMoveRight) :!label _label
    (bind _value (Timeline|타임라인 Play)
      (:Update
        (Transformation|SetRelativeLocation (Variables|Default|GetSphere) (Math|Vector|MakeVector (* _value 1e+02) 0.0 0.0) false false))
      (:Finished
        (Variables|Default|SetIsMoveRight (not (Variables|Default|GetIsMoveRight)))
        (goto _label)))
    (else
      (Timeline|타임라인 Reverse))))

(fn ConstructionScript)

(fn DoPlay
  (|CallParentFunction)
  (CallFunction|EventStart))