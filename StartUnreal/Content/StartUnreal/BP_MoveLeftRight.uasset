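; BP_MoveLeftRight is a Blueprint that moves its Sphere component back and forth along relative X once play is enabled.
; DoPlay calls the parent version and sets IsPlay, which gates the movement in Tick.
; Each Tick steps the offset by a fixed amount without delta time, flipping IsMoveRight past either bound, so speed depends on frame rate.
; BeginPlay and sphere overlaps print debug names.
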(event OnComponentBeginOverlap(Sphere)
  (params (OverlappedComponent :type Primitive%20Component%20Object%20Reference) (OtherActor :type Actor%20Object%20Reference) (OtherComp :type Primitive%20Component%20Object%20Reference) (OtherBodyIndex :type Integer) (bFromSweep :type Boolean) (SweepResult :type Hit%20Result%20Structure%20%28by%20ref%29))
  (Development|PrintString (Utilities|GetDisplayName (Variables|Default|GetSphere))))

(event EventBeginPlay
  (Development|PrintString (Utilities|GetDisplayName self) true true "(R=0.000000,G=0.660000,B=1.000000,A=1.000000)" 6e+01))

(event EventTick
  (params (DeltaSeconds :type Float%20%28single-precision%29))
  (if (Variables|Default|GetIsPlay)
    (if (Variables|Default|GetIsMoveRight)
      ;[1 1 1] 오른쪽 이동
      (Variables|Default|Set거기 (+ (Variables|Default|Get거기) 1.0))
      (Transformation|SetRelativeLocation (Variables|Default|GetSphere) (Math|Vector|MakeVector (Variables|Default|Get거기) 0.0 0.0) false false)
      (if (> (Variables|Default|Get거기) 1e+02)
        (Variables|Default|SetIsMoveRight false))
      (else
        ;[1 1 1] 왼쪽 이동
        (Variables|Default|Set거기 (- (Variables|Default|Get거기) 1.0))
        (Transformation|SetRelativeLocation (Variables|Default|GetSphere) (Math|Vector|MakeVector (Variables|Default|Get거기) 0.0 0.0) false false)
        (if (< (Variables|Default|Get거기) 0.0)
          (Variables|Default|SetIsMoveRight true))))))

(fn ConstructionScript)

(fn DoPlay
  (|CallParentFunction)
  (Variables|Default|SetIsPlay true))