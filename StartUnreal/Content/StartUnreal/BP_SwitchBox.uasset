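; BP_SwitchBox is an overlap-triggered switch that activates a set of other actors.
; When anything begins overlapping its Cube component, it calls DoPlay on every entry in the Actors array, with no filter on the overlapping actor.
; Both begin and end overlap print the involved components and actor for debugging; end overlap does nothing else and reuses the "Begin Overlap" label.
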(event OnComponentBeginOverlap(Cube)
  (params (OverlappedComponent :type Primitive%20Component%20Object%20Reference) (OtherActor :type Actor%20Object%20Reference) (OtherComp :type Primitive%20Component%20Object%20Reference) (OtherBodyIndex :type Integer) (bFromSweep :type Boolean) (SweepResult :type Hit%20Result%20Structure%20%28by%20ref%29))
  (Development|PrintString (Utilities|String|Append "Begin Overlap Overlapped Component : " (Utilities|GetDisplayName OverlappedComponent) ", Other Actor : " (Utilities|GetDisplayName OtherActor) ", Other Comp :" (Utilities|GetDisplayName OtherComp)) true true "(R=0.000000,G=0.660000,B=1.000000,A=1.000000)" 6e+01)
  (for _array_element (Variables|Default|GetActors)
    (Default|DoPlay _array_element)))

(event OnComponentEndOverlap(Cube)
  (params (OverlappedComponent :type Primitive%20Component%20Object%20Reference) (OtherActor :type Actor%20Object%20Reference) (OtherComp :type Primitive%20Component%20Object%20Reference) (OtherBodyIndex :type Integer))
  (Development|PrintString (Utilities|String|Append "Begin Overlap Overlapped Component : " (Utilities|GetDisplayName OverlappedComponent) ", Other Actor : " (Utilities|GetDisplayName OtherActor) ", Other Comp :" (Utilities|GetDisplayName OtherComp)) true true "(R=0.000000,G=0.660000,B=1.000000,A=1.000000)" 6e+01))

(event EventBeginPlay)

(event Collision|EventActorBeginOverlap
  (params (OtherActor :type Actor%20Object%20Reference)))

(event EventTick
  (params (DeltaSeconds :type Float%20%28single-precision%29)))

(fn ConstructionScript)