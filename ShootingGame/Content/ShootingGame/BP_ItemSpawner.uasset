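; BP_ItemSpawner is an item spawner for the shooting game that keeps spawning random pickups at its own transform.
; On BeginPlay, RandItemSpawn spawns a random class from the Items array and binds to the spawned actor's OnDestroyed event.
; When that item is destroyed, EventDestroyItem unbinds and sets a timer to call RandItemSpawn again after a short delay.
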(event EventBeginPlay
  (CallFunction|RandItemSpawn))

(fn ConstructionScript)

(fn RandItemSpawn
  (bind _returnvalue (Game|SpawnActorfromClass (.OutItem (Utilities|Array|Random (Variables|Default|GetItems))) (Transformation|GetActorTransform) "Undefined" "MultiplyWithRoot" 0 0))
  (Game|BindEventtoOnDestroyed _returnvalue (EventDispatchers|CreateEvent :!event EventDestroyItem)))

(fn EventDestroyItem
  (params (DestroyedActor :type Actor%20Object%20Reference))
  (Game|UnbindEventfromOnDestroyed DestroyedActor (EventDispatchers|CreateEvent :!event EventDestroyItem))
  (Utilities|Time|SetTimerbyFunctionName 0 "RandItemSpawn" 5.0))