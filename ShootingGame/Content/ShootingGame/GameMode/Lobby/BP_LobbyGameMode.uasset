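; Lobby game mode for a multiplayer shooting game that gathers players and moves them into the match map.
; BeginPlay sets up a LAN dedicated-server Advanced Session with presence off and a server-name setting.
; Each new player start checks the player count, and once at least two are present a short delay precedes a console servertravel to ThirdPersonMap.
; Join events also carry debug prints, mostly with output switched off.
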(event EventBeginPlay
  (|AdvancedSession (Utilities|Array|MakeArray (Class|AdvancedSessionsLibrary|MakeLiteralSessionPropertyString "ServerName" "ShootingServer")) (Game|GetPlayerController 0) 100 0 true true true false true true false false false true false true))

(event EventPostLogin
  (params (NewPlayer :type Player%20Controller%20Object%20Reference))
  (|CallParentFunction NewPlayer)
  (Development|PrintString (Utilities|String|Append "OnPostLogin - " (Utilities|GetDisplayName NewPlayer)) false false "(R=0.000000,G=0.660000,B=1.000000,A=1.000000)" 6e+01))

(event EventHandleStartingNewPlayer
  (params (NewPlayer :type Player%20Controller%20Object%20Reference))
  (|CallParentFunction NewPlayer)
  (Development|PrintString (Utilities|String|Append "Handle Starting New Player - " (Utilities|GetDisplayName NewPlayer)) false false "(R=0.000000,G=0.660000,B=1.000000,A=1.000000)" 6e+01)
  (bind _returnvalue (Class|GameModeBase|GetNumPlayers))
  (Development|PrintString (Utilities|String|Append "NumPlayers : " (Utilities|String|ToString(Integer) _returnvalue)))
  (if (>= _returnvalue 2)
    (Utilities|FlowControl|Delay 3.0)
    (Development|ExecuteConsoleCommand "servertravel ThirdPersonMap" 0)))

(fn ConstructionScript)