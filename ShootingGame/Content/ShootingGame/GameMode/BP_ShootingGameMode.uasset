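; Game mode for the shooting game that sets up an online session and logs player joins.
; BeginPlay makes an Advanced Sessions call for a LAN dedicated server, using the first player controller and passing a server name as an extra session property.
; PostLogin and HandleStartingNewPlayer call their parents, then print the joining player's name for debugging.
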(event EventHandleStartingNewPlayer
  (params (NewPlayer :type Player%20Controller%20Object%20Reference))
  (|CallParentFunction NewPlayer)
  (Development|PrintString (Utilities|String|Append "Handle Starting New Player - " (Utilities|GetDisplayName NewPlayer))))

(event EventPostLogin
  (params (NewPlayer :type Player%20Controller%20Object%20Reference))
  (|CallParentFunction NewPlayer)
  (Development|PrintString (Utilities|String|Append "OnPostLogin - " (Utilities|GetDisplayName NewPlayer))))

(event EventBeginPlay
  (|CallParentFunction)
  (Development|PrintString "BeginPlay - ShootingGameMode")
  (|AdvancedSession (Utilities|Array|MakeArray (Class|AdvancedSessionsLibrary|MakeLiteralSessionPropertyString "ServerName" "ShootingServer")) (Game|GetPlayerController 0) 100 0 true true true false true true false false false true false true))

(fn ConstructionScript)