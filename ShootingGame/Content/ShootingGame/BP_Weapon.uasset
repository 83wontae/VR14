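; BP_Weapon is a shooting-game gun that characters can pick up, drop, trigger and reload, attaching to a "weapon" socket or detaching with physics.
; Trigger and reload play montages, while shooting spawns muzzle effects and, for the local player, passes camera aim to ReqShoot.
; ReqShoot spends ammo and line-traces from beyond the spring arm, damaging hit Characters.
; An OnRep on Ammo updates the owning player's HUD.
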(event Custom|ReqShoot
  (params (StartLoc :type Vector) (ForwardLoc :type Vector))
  (bind _isused (CallFunction|UseAmmo))
  (if _isused
    (bind (_outhit _returnvalue) (Collision|LineTraceForObjects (+ StartLoc (* ForwardLoc (CallFunction|GetFireStartLength))) (+ StartLoc (* ForwardLoc 5e+03)) (Utilities|Array|MakeArray "ObjectTypeQuery1" "ObjectTypeQuery2" "ObjectTypeQuery3" "ObjectTypeQuery4" "ObjectTypeQuery5" "ObjectTypeQuery6") false 0 "Persistent"))
    (if _returnvalue
      (bind _as캐릭터 (Utilities|Casting|CastToCharacter (.HitActor (Collision|BreakHitResult _outhit))))
      (Game|Damage|ApplyDamage _as캐릭터 1e+01 (Pawn|GetController (Variables|Default|GetOwnChar)) self))))

(fn ConstructionScript)

(fn GetFireStartLength
  (bind _ownchar (Variables|Default|GetOwnChar))
  (bind _returnvalue (Actor|GetComponentbyClass _ownchar "/Script/Engine.SpringArmComponent"))
  (Utilities|IsValid _returnvalue
    (:Is%20Valid
      (return (+ (Variables|/Script/Engine.SpringArmComponent|GetTargetArmLength _returnvalue) 1e+02)))))

(fn UseAmmo
  (if (CallFunction|IsCanShoot)
    (Variables|Default|SetAmmo (- (Variables|Default|GetAmmo) 1))
    (return true)
    (else
      (return false))))

(fn IsCanShoot
  (return (> (Variables|Default|GetAmmo) 0)))

(fn OnRepAmmo
  (Development|PrintString (Utilities|String|Append "Ammo : " (Utilities|String|ToString(Byte) (Variables|Default|GetAmmo))))
  (CallFunction|UpdateMyAmmo (Variables|Default|GetAmmo)))

(fn UpdateMyAmmo
  (params (Ammo :type Byte))
  (bind _returnvalue (Game|GetPlayerController 0))
  (if (== _returnvalue (Pawn|GetController (Variables|Default|GetOwnChar)))
    (bind _asbp_shooting_hud (Utilities|Casting|CastToBP_ShootingHud (HUD|GetHUD _returnvalue)))
    (Default|SetHudAmmo _asbp_shooting_hud Ammo)))

(fn EventDrop
  (params (Character :type Character%20Object%20Reference))
  (bind _staticmesh (Variables|Default|GetStaticMesh))
  (CallFunction|UpdateMyAmmo)
  (Variables|Default|SetOwnChar 0)
  (Physics|SetSimulatePhysics _staticmesh true)
  (Transformation|DetachFromComponent _staticmesh "KeepWorld" "KeepWorld" "KeepWorld" true)
  (return false))

(fn EventPickUp
  (params (Character :type Character%20Object%20Reference))
  (bind _output_get (Variables|Default|SetOwnChar Character))
  (Physics|SetSimulatePhysics (Variables|Default|GetStaticMesh) false)
  (Transformation|AttachComponentToComponent self (Variables|/Script/Engine.Character|GetMesh _output_get) "weapon" "SnapToTarget" "SnapToTarget" "KeepWorld" true)
  (CallFunction|UpdateMyAmmo (Variables|Default|GetAmmo))
  (return false))

(fn EventReload
  (Animation|PlayAnimMontage (Variables|Default|GetOwnChar) (Variables|Default|GetReloadMontage) 1.0 "None")
  (return true))

(fn EventShoot
  (bind _returnvalue (Game|GetPlayerCameraManager 0))
  (bind _staticmesh (Variables|Default|GetStaticMesh))
  (if (CallFunction|IsCanShoot)
    (Effects|SpawnEmitteratLocation "/Game/StarterContent/Particles/P_Explosion.P_Explosion" (Transformation|GetSocketLocation _staticmesh "muzzle") (Transformation|GetSocketRotation _staticmesh "None") "0.100000,0.100000,0.100000")
    (Audio|SpawnSoundatLocation "/Game/StarterContent/Audio/Explosion_Cue.Explosion_Cue" (Transformation|GetSocketLocation (Variables|Default|GetStaticMesh) "muzzle") "0, 0, 0" 1.0 1.0 0.0 0 0)
    (if (== (Variables|Default|GetOwnChar) (Game|GetPlayerCharacter 0))
      (CallFunction|ReqShoot (Camera|GetCameraLocation _returnvalue) (Transformation|GetActorForwardVector _returnvalue))
      (return true))))

(fn EventTrigger
  (Animation|PlayAnimMontage (Variables|Default|GetOwnChar) (Variables|Default|GetShootMontage) 1.0 "None")
  (return true))

(fn IsCanPickUp
  (Utilities|IsValid (Variables|Default|GetOwnChar)
    (:Is%20Valid
      (return false))
    (:Is%20Not%20Valid
      (return true))))